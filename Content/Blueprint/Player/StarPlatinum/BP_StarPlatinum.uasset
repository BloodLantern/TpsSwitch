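; Star Platinum actor, a companion to Jotaro that hovers and fires bullets.
; Each tick it bobs the mesh on a sine of the game mode's TotalTime, offset from the actor's height.
; While ShouldAim is set, it copies Jotaro's camera world rotation into the capsule's relative rotation.
; SpawnBullet spawns a BP_Bullet at the BulletSpawn transform and plays a sound at the actor's location.
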(event Custom|SpawnBullet
  ;[1 1 1] Shoot
  (Game|SpawnActorfromClass "/Game/Blueprint/INeedMoreBullets/BP_Bullet.BP_Bullet_C" (Transformation|GetWorldTransform (Variables|Default|GetBulletSpawn)) "AlwaysSpawn" "MultiplyWithRoot" 0 0)
  (Audio|PlaySoundatLocation "/Game/Assets/Jojo/StarPlatinum/single-ora-bruh.single-ora-bruh" (Transformation|GetActorLocation) "0, 0, 0" 1.0 1.0 0.0 0 0 0 0))

(event EventTick
  (params (DeltaSeconds :type Float%20%28single-precision%29))
  (bind _mesh (Variables|Character|GetMesh))
  (bind _returnvalue (Transformation|GetWorldLocation _mesh))
  ;[1 1 1] Floating effect
  (bind _asbp_base_game_mode (Utilities|Casting|CastToBP_BaseGameMode (Game|GetGameMode)))
  (Transformation|SetWorldLocation (Variables|Character|GetMesh) (Math|Vector|MakeVector (.x _returnvalue) (.y _returnvalue) (- (+ (.z (Transformation|GetActorLocation)) (* (Math|Trig|Sin(Radians) (Variables|/Game/Blueprint/BP_BaseGameMode.BP_BaseGameMode_C|GetTotalTime _asbp_base_game_mode)) 1e+01)) 89.0)) false false)
  (if (Variables|Default|GetShouldAim)
    (bind _asbp_jotaro (Utilities|Casting|CastToBP_Jotaro (Variables|Default|GetJotaro)))
    (Transformation|SetRelativeRotation (Variables|Default|GetCapsuleComponent) (Transformation|GetWorldRotation (Variables|/Game/Blueprint/Player/Jotaro/BP_Jotaro.BP_Jotaro_C|GetCamera _asbp_jotaro)) false false)))

(fn ConstructionScript)