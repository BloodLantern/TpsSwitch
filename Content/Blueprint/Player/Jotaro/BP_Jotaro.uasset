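; BP_Jotaro is the Jotaro player pawn, which constantly moves forward along its control rotation.
; Tick supplies the forward movement, while an input event marked as temporary adds sideways movement from the X axis.
; InitializeStarPlatinum shows the cursor, spawns BP_StarPlatinum at Jotaro's location plus its offset, and notifies it of its owner.
; It then hands the Star Platinum reference to JojoPlayerController.
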(event EventTick
  (params (DeltaSeconds :type Float%20%28single-precision%29))
  (bind _returnvalue (Pawn|GetControlRotation :!class /Script/Engine.Pawn))
  (bind (_roll _pitch _yaw) (Math|Rotator|BreakRotator _returnvalue))
  (Pawn|Input|AddMovementInput (Math|Vector|GetForwardVector (Math|Rotator|MakeRotator _roll _pitch _yaw)) 1.0 false))

(event EventInputMovement
  (params (Value :type Vector%202D%20Structure%20%28by%20ref%29))
  ;[1 1 1] Movement (temporary)
  (Pawn|Input|AddMovementInput (Math|Vector|GetRightVector (Pawn|GetControlRotation :!class /Script/Engine.Pawn)) (.x Value) false))

(fn ConstructionScript)

(fn InitializeStarPlatinum
  (Variables|/Script/Engine.PlayerController|SetbShowMouseCursor (Game|GetPlayerController 0) true)
  (bind _returnvalue (Game|SpawnActorfromClass "/Game/Blueprint/Player/StarPlatinum/BP_StarPlatinum.BP_StarPlatinum_C" (Transformation|GetActorTransform) "Undefined" "MultiplyWithRoot" 0 0))
  (Transformation|SetActorLocation _returnvalue (+ (Transformation|GetActorLocation) (Variables|/Script/TPS_Switch1.PlayerStarPlatinum|GetJotaroOffset _returnvalue)) false false)
  (bind _output_get (Variables|Default|SetStarPlatinum _returnvalue))
  (Class|PlayerStarPlatinum|OnSpawned _output_get self)
  (bind _asjojo_player_controller (Utilities|Casting|CastToJojoPlayerController (Game|GetPlayerController 0)))
  (Variables|/Script/TPS_Switch1.JojoPlayerController|SetStarPlatinum _asjojo_player_controller (Variables|Default|GetStarPlatinum)))