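; BP_BaseGameState is a Blueprint, named as a game state, that spawns furniture props into the level.
; Helper functions SpawnBook, SpawnChair and SpawnTable each spawn their actor class at a given transform and pass the supplied material to its SetMaterial.
; On BeginPlay it spawns a single blue chair at a hard-coded location; the book and table helpers are not called within this Blueprint.
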(event EventBeginPlay
  (CallFunction|SpawnChair (Math|Transform|MakeTransform "5000.000000,1000.000000,0.000000") "/Game/Assets/BlueMaterial.BlueMaterial"))

(event EventTick
  (params (DeltaSeconds :type Float%20%28single-precision%29)))

(fn ConstructionScript)

(fn SpawnBook
  (params (Transform :type Transform) (Material :type Material%20Interface%20Object%20Reference))
  (bind _returnvalue (Game|SpawnActorfromClass "/Game/Blueprint/Obstacles/BP_Book.BP_Book_C" Transform "Undefined" "MultiplyWithRoot" 0 0))
  (Class|Obstacle|SetMaterial _returnvalue Material))

(fn SpawnChair
  (params (Transform :type Transform) (Material :type Material%20Interface%20Object%20Reference))
  (bind _returnvalue (Game|SpawnActorfromClass "/Game/Blueprint/Obstacles/BP_Chair.BP_Chair_C" Transform "Undefined" "MultiplyWithRoot" 0 0))
  (Class|Obstacle|SetMaterial _returnvalue Material))

(fn SpawnTable
  (params (Transform :type Transform) (Material :type Material%20Interface%20Object%20Reference))
  (bind _returnvalue (Game|SpawnActorfromClass "/Game/Blueprint/Obstacles/BP_Table.BP_Table_C" Transform "Undefined" "MultiplyWithRoot" 0 0))
  (Class|Obstacle|SetMaterial _returnvalue Material))