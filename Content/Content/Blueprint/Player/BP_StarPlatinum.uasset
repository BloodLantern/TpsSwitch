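; BP_StarPlatinum is the Star Platinum companion to Jotaro, a floating shooter aimed with an on-screen cursor.
; It creates the BP_Cursor widget and moves it by input, while Tick bobs the mesh on a game-time sine and optionally matches the capsule to Jotaro's camera.
; Shooting deprojects the cursor, traces WorldStatic objects from the camera, and spawns a BP_Bullet aimed at the hit or a far point, with a sound.
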(event Custom|SpawnBullet
  (bind _returnvalue (Game|GetPlayerController 0))
  (bind _returnvalue_2 (Game|GetPlayerCameraManager 0))
  (bind _bulletspawn (Variables|Default|GetBulletSpawn))
  (bind _cursor (Variables|Default|GetCursor))
  (bind _returnvalue_3 (Camera|GetCameraLocation _returnvalue_2))
  (bind _returnvalue_4 (Transformation|GetWorldLocation _bulletspawn))
  (bind _position (Variables|/Game/Blueprint/BP_Cursor.BP_Cursor_C|GetPosition _cursor))
  (bind _worlddirection (Class|PlayerController|DeprojectScreenPositiontoWorld _returnvalue (.x _position) (.y _position)))
  (bind _returnvalue_5 (* _worlddirection 1e+05))
  (bind _returnvalue_6 (+ _returnvalue_3 _returnvalue_5))
  ;[1 1 1] Shoot
  (bind (_outhit _returnvalue_7) (Collision|LineTraceForObjects _returnvalue_3 _returnvalue_6 (Utilities|Array|MakeArray "ObjectTypeQuery1") false 0 "None"))
  (Game|SpawnActorfromClass "/Game/Blueprint/Projectiles/BP_Bullet.BP_Bullet_C" (Math|Transform|MakeTransform _returnvalue_4 (Math|Rotator|FindLookatRotation _returnvalue_4 (Math|Vector|SelectVector (.ImpactPoint (Collision|BreakHitResult _outhit)) _returnvalue_6 _returnvalue_7)) "1.000000,1.000000,1.000000") "AlwaysSpawn" "MultiplyWithRoot" 0 0)
  (Audio|PlaySoundatLocation "/Game/Assets/Jojo/StarPlatinum/single-ora-bruh.single-ora-bruh" (Transformation|GetActorLocation) "0, 0, 0" 1.0 1.0 0.0 0 0 0 0))

(event EventTick
  (params (DeltaSeconds :type Float%20%28single-precision%29))
  (bind _cursor (Variables|Default|GetCursor))
  (bind _mesh (Variables|Character|GetMesh))
  (bind _returnvalue (Transformation|GetWorldLocation _mesh))
  (bind _position (Variables|/Game/Blueprint/BP_Cursor.BP_Cursor_C|GetPosition _cursor))
  ;[1 1 1] Event Tick
  (Utilities|FlowControl|Sequence
    (:then_0
      (bind _asplayer_controller (Utilities|Casting|CastToPlayerController (Pawn|GetController (Variables|Default|GetJotaro))))
      (Transformation|SetRelativeRotation (Variables|Default|GetBulletSpawn) (Math|Rotator|MakeRotator 0.0 (.Pitch (Math|Vector|GetYawPitchfromVector (.WorldDirection (Class|PlayerController|DeprojectScreenPositiontoWorld _asplayer_controller (.x _position) (.y _position))))) (.Yaw (Math|Vector|GetYawPitchfromVector (.WorldDirection (Class|PlayerController|DeprojectScreenPositiontoWorld _asplayer_controller (.x _position) (.y _position)))))) false false))
    (:then_1
      ;;[1 1 1] Floating effect
      (bind _asbp_base_game_mode (Utilities|Casting|CastToBP_BaseGameMode (Game|GetGameMode)))
      (Transformation|SetWorldLocation (Variables|Character|GetMesh) (Math|Vector|MakeVector (.x _returnvalue) (.y _returnvalue) (- (+ (.z (Transformation|GetActorLocation)) (* (Math|Trig|Sin(Radians) (Variables|/Script/TPS_Switch1.BaseGameMode|GetTotalGameTime _asbp_base_game_mode)) 1e+01)) 89.0)) false false))
    (:then_2
      (if (Variables|Default|GetShouldAim)
        (bind _asbp_jotaro (Utilities|Casting|CastToBP_Jotaro (Variables|Default|GetJotaro)))
        (Transformation|SetRelativeRotation (Variables|Default|GetCapsuleComponent) (Transformation|GetWorldRotation (Variables|/Game/Blueprint/Player/BP_Jotaro.BP_Jotaro_C|GetCamera _asbp_jotaro)) false false)))))

(event EventBeginPlay
  ;[1 1 1] Event Begin Play
  (bind _returnvalue (UserInterface|CreateWidget "/Game/Blueprint/BP_Cursor.BP_Cursor_C" (Game|GetPlayerController (.playerid (Variables|Default|GetPlayerData)))))
  (bind _output_get (Variables|Default|SetCursor _returnvalue))
  (UserInterface|Viewport|AddtoViewport _output_get 0))

(event EventMoveCursor
  (params (Value :type Vector%202D%20Structure))
  (bind _returnvalue (* (.y Value) -1.0))
  (bind _returnvalue_2 (Math|Vector2D|MakeVector2D (.x Value) _returnvalue))
  ;[1 1 1] Event Move Cursor
  (if (> (Class|KismetMathLibrary|GetAbsMax2D _returnvalue_2) 0.0)
    (Default|SetPosition (Variables|Default|GetCursor) (+ (Variables|/Game/Blueprint/BP_Cursor.BP_Cursor_C|GetPosition (Variables|Default|GetCursor)) (* _returnvalue_2 (Variables|Default|GetSensitivity))))))

(fn ConstructionScript)