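; BP_Jotaro is the player's Jotaro, adding a health HUD, win and lose screens, and the Star Platinum companion to its parent.
; It creates the health widget on BeginPlay and updates it every Tick.
; OnWin and OnDeath show their result widget, stop the game mode's music and play a voice sound.
; InitializeStarPlatinum shows the cursor, spawns Star Platinum at an offset and registers it with JojoPlayerController.
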(event EventOnDeath
  (|CallParentFunction)
  (bind _returnvalue (UserInterface|CreateWidget "/Game/Blueprint/BP_LoseUI.BP_LoseUI_C"))
  (UserInterface|Viewport|AddtoViewport _returnvalue 0)
  (bind _asbp_base_game_mode (Utilities|Casting|CastToBP_BaseGameMode (Game|GetGameMode)))
  (Audio|Components|Audio|Stop (Variables|/Game/Blueprint/BP_BaseGameMode.BP_BaseGameMode_C|GetMusic _asbp_base_game_mode))
  (Audio|PlaySound2D "/Game/Movies/Defeat/Dio_Muda_Sound.Dio_Muda_Sound" 1.0 1.0 0.0 0 0))

(event EventOnWin
  (|CallParentFunction)
  (bind _returnvalue (UserInterface|CreateWidget "/Game/Blueprint/BP_WinUI.BP_WinUI_C"))
  (UserInterface|Viewport|AddtoViewport _returnvalue 0)
  (bind _asbp_base_game_mode (Utilities|Casting|CastToBP_BaseGameMode (Game|GetGameMode)))
  (Audio|Components|Audio|Stop (Variables|/Game/Blueprint/BP_BaseGameMode.BP_BaseGameMode_C|GetMusic _asbp_base_game_mode))
  (Audio|PlaySound2D "/Game/Movies/Win/Jotaro_Yare_Sound.Jotaro_Yare_Sound" 1.0 1.0 0.0 0 0))

(event EventBeginPlay
  (|CallParentFunction)
  (bind _returnvalue (UserInterface|CreateWidget "/Game/Blueprint/BP_HealthDisplay.BP_HealthDisplay_C"))
  (UserInterface|Viewport|AddtoViewport _returnvalue 0)
  (bind _output_get (Variables|Default|SetHealthDisplay _returnvalue))
  (Variables|/Game/Blueprint/BP_HealthDisplay.BP_HealthDisplay_C|SetJotaro _output_get self))

(event EventTick
  (params (DeltaSeconds :type Float%20%28single-precision%29))
  (|CallParentFunction DeltaSeconds)
  (Default|Update (Variables|Default|GetHealthDisplay)))

(fn ConstructionScript)

(fn InitializeStarPlatinum
  (Variables|/Script/Engine.PlayerController|SetbShowMouseCursor (Game|GetPlayerController 0) true)
  (bind _returnvalue (Game|SpawnActorfromClass "/Game/Blueprint/Player/BP_StarPlatinum.BP_StarPlatinum_C" (Transformation|GetActorTransform) "AlwaysSpawn" "MultiplyWithRoot" 0 0))
  (Transformation|SetActorLocation _returnvalue (+ (Transformation|GetActorLocation) (Variables|/Script/TPS_Switch1.PlayerStarPlatinum|GetJotaroOffset _returnvalue)) false false)
  (bind _output_get (Variables|Default|SetStarPlatinum _returnvalue))
  (Class|PlayerStarPlatinum|OnSpawned _output_get self)
  (bind _asjojo_player_controller (Utilities|Casting|CastToJojoPlayerController (Pawn|GetController)))
  (bind _output_get_2 (Variables|/Script/TPS_Switch1.JojoPlayerController|SetStarPlatinum _asjojo_player_controller _output_get))
  (return _output_get_2))