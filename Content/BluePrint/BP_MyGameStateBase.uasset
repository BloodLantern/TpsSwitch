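; Game state Blueprint that populates the level with a table, a book and a chair when play begins.
; BeginPlay calls a separate spawn function for each prop, placing them in a spaced row high above the world origin.
; Each function spawns its Blueprint actor at the given transform, then passes the supplied material, red in every case, to that actor's SetMaterial.
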(event EventBeginPlay
  (CallFunction|SpawnTable "/Game/Assets/RedMaterial.RedMaterial" (Math|Transform|MakeTransform "0.000000,0.000000,5000.000000"))
  (CallFunction|SpawnBook "/Game/Assets/RedMaterial.RedMaterial" (Math|Transform|MakeTransform "300.000000,0.000000,5000.000000"))
  (CallFunction|SpawnChair "/Game/Assets/RedMaterial.RedMaterial" (Math|Transform|MakeTransform "600.000000,0.000000,5000.000000")))

(event EventTick
  (params (DeltaSeconds :type Float%20%28single-precision%29)))

(fn ConstructionScript)

(fn SpawnChair
  (params (Material :type Material%20Interface%20Object%20Reference) (Transform :type Transform))
  (bind _returnvalue (Game|SpawnActorfromClass "/Game/Blueprint/Obstacles/BP_Chair.BP_Chair_C" Transform "Undefined" "MultiplyWithRoot" 0 0))
  (Class|Obstacle|SetMaterial _returnvalue Material))

(fn SpawnBook
  (params (Material :type Material%20Interface%20Object%20Reference) (Transform :type Transform))
  (bind _returnvalue (Game|SpawnActorfromClass "/Game/Blueprint/Obstacles/BP_Book.BP_Book_C" Transform "Undefined" "MultiplyWithRoot" 0 0))
  (Class|Obstacle|SetMaterial _returnvalue Material))

(fn SpawnTable
  (params (Material :type Material%20Interface%20Object%20Reference) (Transform :type Transform))
  (bind _returnvalue (Game|SpawnActorfromClass "/Game/Blueprint/Obstacles/BP_Table.BP_Table_C" Transform "Undefined" "MultiplyWithRoot" 0 0))
  (Class|Obstacle|SetMaterial _returnvalue Material))