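; Player-controlled Star Platinum character with a floating idle effect, mouse look and an aim mode.
; Adds its Enhanced Input mapping context on begin play, feeding look input to controller yaw and pitch.
; Each tick bobs the mesh around the actor's height using a sine of BaseGameMode's total time.
; Right mouse switches mesh animations between aim and punch while a timeline moves the spring arm's length and socket offset, reversing on release.
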(event Input|EnhancedActionEvents|EnhancedInputActionLookAround
  (params (ActionValue :type Vector%202D%20Structure) (ElapsedSeconds :type Float%20%28double-precision%29) (TriggeredSeconds :type Float%20%28double-precision%29) (InputAction :type Input%20Action%20Object%20Reference :default "/Game/BluePrint/Characters/StarPlatinum/LookAround.LookAround"))
  ;[1 1 1] Camera
  (:Triggered
    (Pawn|Input|AddControllerYawInput (.x ActionValue))
    (Pawn|Input|AddControllerPitchInput (.y ActionValue))))

(event EventTick
  (params (DeltaSeconds :type Float%20%28single-precision%29))
  (bind _mesh (Variables|Character|GetMesh))
  (bind _returnvalue (Transformation|GetWorldLocation _mesh))
  ;[1 1 1] Floatin effect
  (bind _asbase_game_mode (Utilities|Casting|CastToBaseGameMode (Game|GetGameMode)))
  (Transformation|SetWorldLocation (Variables|Character|GetMesh) (Math|Vector|MakeVector (.x _returnvalue) (.y _returnvalue) (- (+ (.z (Transformation|GetActorLocation)) (* (Math|Trig|Sin(Radians) (Variables|/Game/BluePrint/BaseGameMode.BaseGameMode_C|GetTotalTime _asbase_game_mode)) 1e+01)) 89.0)) false false))

(event EventBeginPlay
  (bind _returnvalue (Game|GetPlayerController 0))
  (bind _returnvalue_2 (PlayerController|LocalPlayerSubsystems|GetEnhancedInputLocalPlayerSubsystem _returnvalue))
  (Utilities|IsValid _returnvalue_2
    (:Is%20Valid
      (Input|AddMappingContext _returnvalue_2 "/Game/BluePrint/Characters/StarPlatinum/IMC_StarPlatinum.IMC_StarPlatinum" 0 "(bIgnoreAllPressedKeysUntilRelease=True,bForceImmediately=False)"))))

(event Input|MouseEvents|RightMouseButton
  (params (Key :type Key%20Structure :default "None"))
  (:Pressed
    (Components|Animation|PlayAnimation (Variables|Character|GetMesh) "/Game/Jojo/StarPlatinum/starplatinum_aim_Anim1.starplatinum_aim_Anim1" false)
    (bind (_direction _lengh _socketoffset) (Timeline|AimingSystem Play)
      (:Update
        (Variables|/Script/Engine.SpringArmComponent|SetTargetArmLength (Variables|Default|GetSpringArm) _lengh)
        (Variables|/Script/Engine.SpringArmComponent|SetSocketOffset (Variables|Default|GetSpringArm) _socketoffset))))
  (:Released
    (Components|Animation|PlayAnimation (Variables|Character|GetMesh) "/Game/Jojo/StarPlatinum/starplatinum_punch_Anim.starplatinum_punch_Anim" false)
    (Timeline|AimingSystem Reverse)))

(fn ConstructionScript)